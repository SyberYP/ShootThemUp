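; Game instance Blueprint that hosts and joins online multiplayer sessions through the async session nodes.
; StartSession creates a non-LAN session and, on success, opens CubeLevel_2x2 as a listen server.
; JoinSession searches for non-LAN sessions and joins the first result if any are found, with no failure handling on either path.
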(event Custom|JoinSession
  (bind _results (|FindSessions (Game|GetPlayerController 0) 10 false)
    (:OnSuccess
      (if (> (Utilities|Array|Length _results) 0)
        (|JoinSession (Game|GetPlayerController 0) (Utilities|Array|Get(acopy) _results))))))

(event Custom|StartSession
  (|Session (Game|GetPlayerController 0) 10 false
    (:OnSuccess
      (Game|OpenLevel(byObjectReference) "/Game/Levels/CubeLevel_2x2.CubeLevel_2x2" true "Listen"))))