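; AI character Blueprint child, apparently of an STU AI character, with a helper for finding the nearest TargetPoint.
; GetClosestTargetPoint scans all TargetPoint actors and keeps the closest by distance, using MinimumDistance without resetting it in the function.
; The AIMoveTo toward that point is disconnected and never runs.
; BeginPlay is empty with its parent call unwired, and BehaviorTreeAsset is unused in the graph.
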(event EventBeginPlay)

(event Collision|EventActorBeginOverlap
  (params (OtherActor :type Actor%20Object%20Reference))
  (|CallParentFunction OtherActor) ; This node is disabled and will not be called.\nDrag off pins to build functionality.
)

(event EventTick
  (params (DeltaSeconds :type Float%20%28single-precision%29))
  (|CallParentFunction DeltaSeconds) ; This node is disabled and will not be called.\nDrag off pins to build functionality.
)

(fn ConstructionScript
  (|CallParentFunction))

(fn GetClosestTargetPoint
  (bind _outactors (Actor|GetAllActorsOfClass "/Script/Engine.TargetPoint"))
  (for _array_element _outactors
    (if (< (Math|Vector|VectorLength (- (Transformation|GetActorLocation) (Transformation|GetActorLocation _array_element))) (LocalVariables|GetMinimum%20distance))
      (LocalVariables|SetMinimum%20distance (Math|Vector|VectorLength (- (Transformation|GetActorLocation) (Transformation|GetActorLocation _array_element))))
      (LocalVariables|SetClosest%20Target _array_element)))
  (return (LocalVariables|GetClosest%20Target)))